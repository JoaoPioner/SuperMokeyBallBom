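; Player pawn for a physics ball that rolls with Enhanced Input, pushes simulating objects on hit and counts collected coins.
; Move input becomes camera-yaw-relative torque, applied locally and sent through a movement RPC, with linear damping added on release.
; Movement also tilts the camera for feedback, while look input only turns yaw.
; Falling below a height threshold respawns it at the first PlayerStart; FullStop disables input and zeroes velocity.
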(event `self.ReceiveBeginPlay`
  ; Troca Controller
  (bind _asplayer_controller (cast `PlayerController` (`self.GetController`)))
  (`EnhancedInputSubsystemInterface.AddMappingContext` (pcsubsystem `EnhancedInputLocalPlayerSubsystem` _asplayer_controller) "/Game/InputMap/IA_Player_InputMappingContext.IA_Player_InputMappingContext" 0 (struct)))

(event `self.Bola.OnComponentHit`
  (params (HitComponent :type "PrimitiveComponent Object Reference") (OtherActor :type "Actor Object Reference") (OtherComp :type "PrimitiveComponent Object Reference") (NormalImpulse :type "Vector Structure") (Hit :type "HitResult Structure (by ref)"))
  ; Adicionar impulso na hora de bater na parede
  (if (`SceneComponent.IsSimulatingPhysics` OtherComp "None")
    (`PrimitiveComponent.AddImpulseAtLocation` OtherComp (* (`self.GetVelocity`) (`self.PushStrenght`)) (`self.K2_GetActorLocation`) "None")))

(event `EnhancedInput|/Game/InputMap/IA_Move`
  (params (ActionValue :type "Vector2D Structure") (ElapsedSeconds :type "Float (double-precision)") (TriggeredSeconds :type "Float (double-precision)") (InputAction :type "InputAction Object Reference" :default "/Game/InputMap/IA_Move.IA_Move"))
  ; Tilta a camera (teclado)
  (:`Triggered`
    (`SceneComponent.K2_SetRelativeRotation` (`self.Camera`) (`KismetMathLibrary.RInterpTo_Constant` (`SceneComponent.RelativeRotation` (`self.Camera`)) (`KismetMathLibrary.ComposeRotators` (* (`KismetMathLibrary.NegateRotator` (`KismetMathLibrary.MakeRotator` ActionValue_X)) 100.0) (* (`KismetMathLibrary.NegateRotator` (`KismetMathLibrary.MakeRotator` 0.0 ActionValue_Y)) 15.0)) (`GameplayStatics.GetWorldDeltaSeconds`) 15.0) false false))
  (:`Completed`
    (`SceneComponent.K2_SetRelativeRotation` (`self.Camera`) (`KismetMathLibrary.RInterpTo_Constant` (`SceneComponent.RelativeRotation` (`self.Camera`)) (`KismetMathLibrary.MakeRotator` 0.0 -25.0) (`GameplayStatics.GetWorldDeltaSeconds`) 10.0) false false)))

(event `self.ReceiveControllerChanged`
  (params (OldController :type "Controller Object Reference") (NewController :type "Controller Object Reference"))
  ; Troca Controller
  (bind _asplayer_controller (cast `PlayerController` NewController))
  (bind _returnvalue (pcsubsystem `EnhancedInputLocalPlayerSubsystem` _asplayer_controller))
  (`/Engine/EditorBlueprintResources/StandardMacros.IsValid` _returnvalue
    (:`Is Valid`
      (`EnhancedInputSubsystemInterface.AddMappingContext` _returnvalue "/Game/InputMap/IA_Player_InputMappingContext.IA_Player_InputMappingContext" 0 (struct)))))

(event `FullStop`
  ; Para o player
  (`self.DisableInput` (`GameplayStatics.GetPlayerController` 0))
  (`PrimitiveComponent.SetPhysicsLinearVelocity` (`self.Bola`) (0.0 0.0 0.0) false "None")
  (`PrimitiveComponent.SetPhysicsAngularVelocityInDegrees` (`self.Bola`) (0.0 0.0 0.0) false "None")
  (set `self.Strenght` (0.0 0.0 0.0)))

(event `EnhancedInput|/Game/InputMap/IA_Look`
  (params (ActionValue :type "Vector2D Structure") (ElapsedSeconds :type "Float (double-precision)") (TriggeredSeconds :type "Float (double-precision)") (InputAction :type "InputAction Object Reference" :default "/Game/InputMap/IA_Look.IA_Look"))
  ; move camera (mouse)
  (:`Triggered`
    (`self.AddControllerYawInput` ActionValue_X)))

(event `EnhancedInput|/Game/InputMap/IA_Move`
  (params (ActionValue :type "Vector2D Structure") (ElapsedSeconds :type "Float (double-precision)") (TriggeredSeconds :type "Float (double-precision)") (InputAction :type "InputAction Object Reference" :default "/Game/InputMap/IA_Move.IA_Move"))
  (bind _mvspeed (`self.MvSpeed`))
  (bind (_returnvalue_roll _returnvalue_pitch _returnvalue_yaw) (`KismetMathLibrary.BreakRotator` (`Controller.GetControlRotation` (`GameplayStatics.GetPlayerController` 0))))
  (bind _returnvalue (`KismetMathLibrary.MakeRotator` 0.0 0.0 _returnvalue_yaw))
  ;[1 1 1] CALCULA MOV STR
  (:`Triggered`
    (bind _output_get (set `self.Strenght` (+ (* (* (`KismetMathLibrary.GetRightVector` _returnvalue) ActionValue_Y 1) _mvspeed) (* (* (`KismetMathLibrary.GetForwardVector` _returnvalue) ActionValue_X -1) _mvspeed))))
    (`self.ApplyMovementForce` _output_get)
    (`self.RPC_MOVEMENT` _output_get))
  (:`Completed`
    (`self.ApplyMovementForce` (0.0 0.0 0.0) 3.0)
    (`self.RPC_MOVEMENT` (0.0 0.0 0.0) 3.0)))

(event `self.ReceiveTick`
  (params (DeltaSeconds :type "Float (single-precision)"))
  ; FallOff Check
  (if (< (.z (`SceneComponent.K2_GetComponentLocation` (`self.Bola`))) -1000.0)
    (`GameplayStatics.PlaySound2D` "/Game/Blueprints/Sounds/Stings_Death/417486__mentoslat__8-bit-death-sound.417486__mentoslat__8-bit-death-sound" 1.0 1.0 0.0 null null)
    (`self.ServerRespawn`)))

(event `RPC_MOVEMENT`
  (params (MoveStrVector :type "Vector Structure") (newDamping :type "Float (double-precision)"))
  ; RPC MOVEMENT
  (`self.ApplyMovementForce` MoveStrVector newDamping))

(event `ServerRespawn`
  (bind _bola (`self.Bola`))
  (bind _outactors (`GameplayStatics.GetAllActorsOfClass` "/Script/Engine.PlayerStart"))
  (`self.K2_SetActorLocation` (`self.K2_GetActorLocation` (`|GetArrayItem` _outactors)) false true)
  (`self.K2_SetActorRotation` (struct))
  (`PrimitiveComponent.SetPhysicsLinearVelocity` _bola (0.0 0.0 0.0) false "None")
  (`PrimitiveComponent.SetPhysicsAngularVelocityInRadians` _bola (0.0 0.0 0.0) false "None")
  (`SceneComponent.K2_SetRelativeRotation` :`self` (`self.Camera`)))

(event `ApplyMovementForce`
  (params (ForceVector :type "Vector Structure") (newDamping :type "Float (double-precision)"))
  ; RPC MOVEMENT
  (`PrimitiveComponent.SetLinearDamping` (`self.Bola`) newDamping)
  (`PrimitiveComponent.AddTorqueInRadians` (`self.Bola`) ForceVector "None" true))

(fn `addCoin`
  (`GameplayStatics.PlaySound2D` "/Game/Blueprints/Sounds/Stings_CoinPickup/341695__aceofspadesproduc100__coins-1.341695__aceofspadesproduc100__coins-1" 1.0 1.0 0.0 null null)
  (set `self.CoinCount` (+ (`self.CoinCount`) 1)))

(fn `UserConstructionScript`)