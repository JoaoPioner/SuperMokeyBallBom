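; BP_TiltWorld is an actor that tilts itself from player input, apparently as the world for a ball pawn.
; On BeginPlay it spawns BP_BallPawn at BallSpawn, has player controller 0 possess it, and enables input on itself.
; Each tick it scales forward and right tilt axes by MaxTiltAngle, eases pitch and roll toward them with FInterpTo, then sets its rotation with zero yaw and no physics teleport.
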(event `self.ReceiveTick`
  (params (DeltaSeconds :type "Float (single-precision)"))
  (set `self.TargetPitch` (* (`self.GetInputAxisValue`) (`self.MaxTiltAngle`)))
  (set `self.TargetRoll` (* (`self.GetInputAxisValue`) (`self.MaxTiltAngle`)))
  (set `self.CurrentPitch` (`KismetMathLibrary.FInterpTo` (`self.CurrentPitch`) (`self.TargetPitch`) (`GameplayStatics.GetWorldDeltaSeconds`) (`self.TiltSpeed`)))
  (set `self.CurrentRoll` (`KismetMathLibrary.FInterpTo` (`self.CurrentRoll`) (`self.TargetRoll`) (`GameplayStatics.GetWorldDeltaSeconds`) (`self.TiltSpeed`)))
  (`self.K2_SetActorRotation` (`KismetMathLibrary.MakeRotator` (`self.CurrentRoll`) (`self.CurrentPitch`))))

(event `self.ReceiveBeginPlay`
  (bind _returnvalue (`|SpawnActorFromClass` "/Game/Blueprints/BP_BallPawn.BP_BallPawn_C" (`SceneComponent.K2_GetComponentToWorld` (`self.BallSpawn`)) "Undefined" "MultiplyWithRoot" null null))
  (set `self.BallPawnRef` _returnvalue)
  (`Controller.Possess` (`GameplayStatics.GetPlayerController` 0) (`self.BallPawnRef`))
  (`self.EnableInput` (`GameplayStatics.GetPlayerController` 0)))

(fn `UserConstructionScript`)